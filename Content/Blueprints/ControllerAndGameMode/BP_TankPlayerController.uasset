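; BP_TankPlayerController is the player controller for the tank game, setting up the camera view and input when play begins.
; On BeginPlay it switches the view target to the first CameraActor found in the level, if any exists.
; It then gets the first player pawn's controller and adds the IMC_NewMovement mapping context to its Enhanced Input local player subsystem.
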(event EventBeginPlay
  (Utilities|FlowControl|Sequence
    (:then_0
      (bind _outactors (Actor|GetAllActorsOfClass "/Script/Engine.CameraActor"))
      (if (> (Utilities|Array|Length _outactors) 0)
        (Game|Player|SetViewTargetwithBlend (Utilities|Array|Get(acopy) _outactors) 0.0 "VTBlend_Linear" 0.0 false)))
    (:then_1
      (bind _asplayer_controller (Utilities|Casting|CastToPlayerController (Pawn|GetController (Game|Player|GetPlayerPawn 0))))
      (Utilities|IsValid (PlayerController|LocalPlayerSubsystems|GetEnhancedInputLocalPlayerSubsystem _asplayer_controller)
        (:Is%20Valid
          (Input|AddMappingContext (PlayerController|LocalPlayerSubsystems|GetEnhancedInputLocalPlayerSubsystem _asplayer_controller) "/Game/Blueprints/Input/IMC_NewMovement.IMC_NewMovement" 0 "(bIgnoreAllPressedKeysUntilRelease=True,bForceImmediately=False,bNotifyUserSettings=False)"))))))

(fn ConstructionScript)